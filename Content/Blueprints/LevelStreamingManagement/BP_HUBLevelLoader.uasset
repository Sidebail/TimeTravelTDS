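; Hub trigger actor that swaps streamed levels behind fog of war when the player first overlaps it.
; A timeline fades fog in on the unload-side meshes, then blocking-unloads the previous level if one is named.
; A reversed timeline then clears the load-side fog, and its first update moves the next level to a transform point and streams it in.
; Both fog sides use dynamic M_FogOfWar materials created at BeginPlay.
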(event `self.ReceiveBeginPlay`
  (`|ExecutionSequence`
    (:`then_0`
      ;[1 1 1] Set up Dynamic Material Instances for FogOfWar meshes
      (bind _returnvalue (`KismetMaterialLibrary.CreateDynamicMaterialInstance` "/Game/Enviroment/Materials/M_FogOfWar.M_FogOfWar"))
      (bind _output_get (set `self.UnloadFogOfWarMaterial` _returnvalue))
      (`MaterialInstanceDynamic.SetVectorParameterValue` _output_get "Color" (`KismetMathLibrary.MakeColor` 0.0 0.0 0.0 0.0))
      (bind _returnvalue_2 (`KismetMaterialLibrary.CreateDynamicMaterialInstance` "/Game/Enviroment/Materials/M_FogOfWar.M_FogOfWar"))
      (`MaterialInstanceDynamic.SetVectorParameterValue` _returnvalue_2 "Color" (`KismetMathLibrary.MakeColor` 0.0))
      (set `self.LoadFogOfWarMaterial` _returnvalue_2)
      (for _array_element (`self.UnloadForOfWarMeshes`)
        (`PrimitiveComponent.SetMaterial` (`StaticMeshActor.StaticMeshComponent` _array_element) 0 _output_get)))
    (:`then_1`
      (for _array_element_2 (`self.LoadForOfWarMeshes`)
        (`PrimitiveComponent.SetMaterial` (`StaticMeshActor.StaticMeshComponent` _array_element_2) 0 (`self.LoadFogOfWarMaterial`))))
    (:`then_2`
      (for _array_element_3 (`self.UnloadForOfWarMeshes`)
        (`PrimitiveComponent.SetMaterial` (`StaticMeshActor.StaticMeshComponent` _array_element_3) 0 (`self.UnloadFogOfWarMaterial`))))))

(event `self.ReceiveActorBeginOverlap`
  (params (OtherActor :type "Actor Object Reference"))
  (bind _returnvalue (`KismetStringLibrary.Conv_StringToName` (`KismetTextLibrary.Conv_TextToString` (`self.PreviousLevelName`))))
  (bind _returnvalue_2 (`KismetStringLibrary.Conv_StringToName` (`KismetTextLibrary.Conv_TextToString` (`self.NextLevelName`))))
  ;[1 0 0] Main Logic for Loading/Unloading Levels using LevelStreaming and LevelTransforms
  (cast `/Game/Blueprints/PlayerCharacter/BP_PlayerCharacter` OtherActor)
  (`/Engine/EditorBlueprintResources/StandardMacros.DoOnce` false
    (:`Completed`
      ;;[1 1 1] Turn on the FogOfWar from left side
      (bind (_direction _alpha) (`Timeline|FogFadeOut`)
        (:`Update`
          (`MaterialInstanceDynamic.SetVectorParameterValue` (`self.UnloadFogOfWarMaterial`) "Color" (`KismetMathLibrary.MakeColor` 0.0 0.0 0.0 _alpha)))
        (:`Finished`
          (if (or (== _returnvalue "None") (== _returnvalue "None"))
            (bind (_direction_2 _alpha_2) (`Timeline|FogFadeIn` :!via `ReverseFromEnd` :!label _label)
              (:`Update`
                (`MaterialInstanceDynamic.SetVectorParameterValue` (`self.LoadFogOfWarMaterial`) "Color" (`KismetMathLibrary.MakeColor` 0.0 0.0 0.0 _alpha_2))
                (`/Engine/EditorBlueprintResources/StandardMacros.DoOnce` false
                  (:`Completed`
                    (bind _output_get (set `LevelStreaming.LevelTransform` (`self.GetTransform` (`self.NextLevelTransformPoint`)) (`GameplayStatics.GetStreamingLevel` _returnvalue_2)))
                    (`GameplayStatics.LoadStreamLevel` _returnvalue_2 true)
                    (`KismetSystemLibrary.PrintString` (`KismetStringLibrary.Conv_TransformToString` _output_get))))))
            (else
              (`GameplayStatics.UnloadStreamLevel` _returnvalue true)
              (goto _label :!via `ReverseFromEnd`))))))))

(fn `UserConstructionScript`)