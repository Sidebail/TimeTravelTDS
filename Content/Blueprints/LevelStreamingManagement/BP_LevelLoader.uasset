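; Trigger actor that swaps streamed levels the first time BP_PlayerCharacter overlaps it.
; If a level to load is named, it first unloads any named old level with blocking.
; It then moves the new streaming level to NewLevelPoint's transform and loads it without blocking, visible once loaded.
; An author note warns that the repositioning fails in PIE and needs standalone play.
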(event `self.ReceiveActorBeginOverlap`
  (params (OtherActor :type "Actor Object Reference"))
  (bind _returnvalue (`KismetStringLibrary.Conv_StringToName` (`KismetTextLibrary.Conv_TextToString` (`self.LevelNameToLoad`))))
  (cast `/Game/Blueprints/PlayerCharacter/BP_PlayerCharacter` OtherActor)
  (`/Engine/EditorBlueprintResources/StandardMacros.DoOnce` false
    (:`Completed`
      (if (`KismetTextLibrary.NotEqual_TextText` (`self.LevelNameToLoad`) "None")
        (if (`KismetTextLibrary.NotEqual_TextText` (`self.LevelNameToUnload`) "None")
          (`GameplayStatics.UnloadStreamLevel` (`KismetStringLibrary.Conv_StringToName` (`KismetTextLibrary.Conv_TextToString` (`self.LevelNameToUnload`))) true))
        ;[1 1 1] DOESNT WORK IN PIE! Use Play As Standalone PIE
        (set `LevelStreaming.LevelTransform` (`self.GetTransform` (`self.NewLevelPoint`)) (`GameplayStatics.GetStreamingLevel` _returnvalue))
        (`GameplayStatics.LoadStreamLevel` _returnvalue true)))))

(fn `UserConstructionScript`)