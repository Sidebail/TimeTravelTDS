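; BP_DoorSystem is a swinging door that opens and closes automatically through two trigger volumes.
; Overlapping EnterTrigger opens it and overlapping ExitTrigger closes it, with an IsDoorOpen flag guarding against repeat calls.
; The OpenDoor timeline plays forward or in reverse, and its track is remapped to DoorAngleOrHeight to set the relative yaw of DoorPart.
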(event `Opening`
  (if (not (`self.bIsDoorOpen`))
    (set `self.bIsDoorOpen` true)
    (bind (_direction _doorrotationz_yaw) (`Timeline|OpenDoor` :!label _label)
      (:`Update`
        (`SceneComponent.K2_SetRelativeRotation` (`self.DoorPart`) (`KismetMathLibrary.MakeRotator` 0.0 0.0 (`KismetMathLibrary.MapRangeClamped` _doorrotationz_yaw 0.0 1.0 0.0 (`self.DoorAngleOrHeight`))) false false)))))

(event `Closing`
  (if (`self.bIsDoorOpen`)
    (set `self.bIsDoorOpen` false)
    (goto _label :!via `Reverse`)))

(event `self.EnterTrigger.OnComponentBeginOverlap`
  (params (OverlappedComponent :type "PrimitiveComponent Object Reference") (OtherActor :type "Actor Object Reference") (OtherComp :type "PrimitiveComponent Object Reference") (OtherBodyIndex :type Integer) (bFromSweep :type Boolean) (SweepResult :type "HitResult Structure (by ref)"))
  (`self.Opening`))

(event `self.ExitTrigger.OnComponentBeginOverlap`
  (params (OverlappedComponent :type "PrimitiveComponent Object Reference") (OtherActor :type "Actor Object Reference") (OtherComp :type "PrimitiveComponent Object Reference") (OtherBodyIndex :type Integer) (bFromSweep :type Boolean) (SweepResult :type "HitResult Structure (by ref)"))
  (`self.Closing`))

(fn `UserConstructionScript`)