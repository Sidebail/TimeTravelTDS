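; Top-down player character Blueprint that handles sprint, aim, jump and camera input, with the spring arm configured in the construction script.
; Sprint and aim call ChangeMovementState, with sprint checking whether velocity matches facing, and aiming also shifts the boom forward by SightRange.
; Zoom changes arm length within height limits, then continues it through a looping timer that blocks further input until done.
; Tick's state switch is empty, and reload, fire-montage and stick-look logic is stubbed or disconnected.
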(event `InputAxis|SprintAxis`
  (params (AxisValue :type "Float (single-precision)"))
  (if (> AxisValue 0.0)
    (if (== (`KismetMathLibrary.Normal` (`self.GetVelocity`)) (`KismetMathLibrary.Normal` (`self.GetActorForwardVector`)) :`ErrorTolerance` 0.3)
      (`self.ChangeMovementState` "RUN_STATE")
      (else
        (`self.ChangeMovementState` "WALK_STATE")))))

(event `InputAxis|Zoom`
  (params (AxisValue :type "Float (single-precision)"))
  (`self.CameraSlide` AxisValue))

(event `InputAction|Fire`
  (params (Key :type "Key Structure")))

(event `InputAction|Aim`
  (params (Key :type "Key Structure"))
  (:`Pressed`
    (`self.ToggleAiming` true))
  (:`Released`
    (`self.ToggleAiming` false)))

(event `Key|F`
  (params (Key :type "Key Structure"))
  (:`Pressed`
    (`self.Shot Shake`)))

(event `InputAction|JumpAction`
  (params (Key :type "Key Structure"))
  (:`Pressed`
    (`self.Jump`)
    (`|PlayMontage` (`self.Mesh`) "/Game/Mannequin/Animations/NewAnimations/NewJump_From_Stand_Montage.NewJump_From_Stand_Montage")))

(event `self.ReceiveTick`
  (params (DeltaSeconds :type "Float (single-precision)"))
  (`|ExecutionSequence`
    (:`then_0`
      (bind _returnvalue (`self.GetCursorToWorld`))
      (set `self.ClampedCameraHeight` (`KismetMathLibrary.MapRangeClamped` (`SpringArmComponent.TargetArmLength` (`self.CameraBoom`)) (`self.CameraHeightMin`) (`self.CameraHeightMax`) 0.5 1.0))
      (set `self.DistanceCameraBoomChar` (`KismetMathLibrary.VSizeXY` (- (`SceneComponent.K2_GetComponentLocation` (`self.CapsuleComponent`)) _returnvalue)))
      (switch `EMovementState` (`self.MovementState`)))))

(event `self.WeaponReloadStart_BP`
  (params (Anim :type "AnimMontage Object Reference")))

(event `self.WeaponReloadEnd_BP`
  (`KismetSystemLibrary.PrintString` "2"))

(fn `CameraSlide`
  (params (Value :type "Float (double-precision)"))
  (bind _returnvalue (- (`SpringArmComponent.TargetArmLength` (`self.CameraBoom`)) (`self.CameraHeightZoomValue`)))
  (bind _returnvalue_2 (+ (`SpringArmComponent.TargetArmLength` (`self.CameraBoom`)) (`self.CameraHeightZoomValue`)))
  (if (`self.SlideDone`)
    (if (!= Value 0.0)
      (if (< Value 0.0)
        (if (>= (`self.CameraHeightMax`) _returnvalue_2)
          (set `SpringArmComponent.TargetArmLength` _returnvalue_2 (`self.CameraBoom`))
          (set `self.SlideUp` true)
          (set `self.SlideDone` false :!label _label)
          (bind _returnvalue_3 (`KismetSystemLibrary.K2_SetTimer` null "CameraSlideSmoothTick" (`self.CameraTimerTick`) true))
          (set `self.CameraZoomTimerHandle` _returnvalue_3))
        (elif (<= (`self.CameraHeightMin`) _returnvalue)
          (set `SpringArmComponent.TargetArmLength` _returnvalue (`self.CameraBoom`))
          (set `self.SlideUp` false)
          (goto _label))))))

(fn `CameraSlideSmoothTick`
  (bind _cameraboom (`self.CameraBoom`))
  (bind _cameraheightzoomstepvalue (`self.CameraHeightZoomStepValue`))
  (bind _targetarmlength (`SpringArmComponent.TargetArmLength` _cameraboom))
  (set `self.CurrentSlideDistance` (+ (`self.CurrentSlideDistance`) _cameraheightzoomstepvalue))
  (set `SpringArmComponent.TargetArmLength` (select `bool` (`self.SlideUp`) :`false` (- _targetarmlength _cameraheightzoomstepvalue) :`true` (+ _targetarmlength _cameraheightzoomstepvalue)) _cameraboom)
  (if (>= (`self.CurrentSlideDistance`) (`self.CameraHeightZoomValue`))
    (set `self.CurrentSlideDistance` 0.0)
    (set `self.SlideDone` true)
    (`KismetSystemLibrary.K2_ClearAndInvalidateTimerHandle` (`self.CameraZoomTimerHandle`))))

(fn `Shot Shake`
  (`GameplayStatics.PlayWorldCameraShake` "/Game/Blueprints/Game/BP_ShootShakeCamera.BP_ShootShakeCamera_C" (`SceneComponent.K2_GetComponentLocation` (`self.TopDownCameraComponent`)) 0.0 30.0))

(fn `ToggleAiming`
  (params (bIsAimEnabled :type Boolean))
  (`SceneComponent.K2_SetRelativeLocation` (`self.CameraBoom`) (`KismetMathLibrary.MakeVector` (`KismetMathLibrary.SelectFloat` (`self.SightRange`) 0.0 bIsAimEnabled)) false false)
  (if bIsAimEnabled
    (`self.ChangeMovementState` "AIM_STATE")
    (else
      (`self.ChangeMovementState` "WALK_STATE"))))

(fn `UserConstructionScript`
  (bind _cameraboom (`self.CameraBoom`))
  (set `SpringArmComponent.TargetArmLength` (`self.Height`) _cameraboom)
  (`SceneComponent.K2_SetRelativeRotation` _cameraboom (`self.RotateCamera`) false false)
  (set `SpringArmComponent.bEnableCameraLag` (`self.Flow`) _cameraboom)
  (set `SpringArmComponent.CameraLagSpeed` (`self.CoefSmoth`) _cameraboom))