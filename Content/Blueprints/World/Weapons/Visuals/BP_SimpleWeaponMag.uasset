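; BP_SimpleWeaponMag is a visual weapon magazine prop that shrinks itself after a set lifetime.
; BeginPlay starts a one-shot CaseLifetime timer that sets IsShrinking.
; Tick then scales MagBase down uniformly at a constant rate toward 0.01, using its X scale for all axes.
; DestroyActor waits for a scale of 0.005 or less, below that interpolation target, so shrinking alone does not reach it.
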(event `self.ReceiveBeginPlay`
  (`KismetSystemLibrary.K2_SetTimerDelegate` (delegate `ShrinkAndDestroy`) (`self.CaseLifetime`)))

(event `ShrinkAndDestroy`
  (set `self.bIsShrinking` true))

(event `self.ReceiveTick`
  (params (DeltaSeconds :type "Float (single-precision)"))
  (bind _magbase (`self.MagBase`))
  (bind _returnvalue_x (`KismetMathLibrary.BreakVector` (`SceneComponent.K2_GetComponentScale` _magbase)))
  (bind _returnvalue (`KismetMathLibrary.FInterpTo_Constant` _returnvalue_x 0.01 DeltaSeconds 0.05))
  (if (`self.bIsShrinking`)
    (`SceneComponent.SetWorldScale3D` _magbase (`KismetMathLibrary.MakeVector` _returnvalue _returnvalue _returnvalue))
    (if (<= _returnvalue_x 0.005)
      (`self.K2_DestroyActor`))))

(fn `UserConstructionScript`)